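; Base hat collectible that the player picks up and wears, and that can be moved onto an NPC.
; While collectable, a player overlap notifies the game mode once, removes the sphere, snaps the hat to the player's Hat component and fades an audio parameter through a timeline.
; Separate events detach the mesh or attach it to an NPC's Hat socket.
; A load event restores the collected state with a grey material and no sphere or audio.
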(event `Load Collected State`
  (set `self.CollectableMode` false)
  (`PrimitiveComponent.SetMaterial` (`self.StaticMesh`) 0 "/Engine/EditorMeshes/ColorCalibrator/M_GreyBall.M_GreyBall") ; Pick whatever material says \n"i'm collected already" to you.
  (`KismetSystemLibrary.PrintString` "Collected State Loadedd")
  (`ActorComponent.K2_DestroyComponent` (`self.Sphere`))
  (`ActorComponent.K2_DestroyComponent` (`self.001_Scene_2_-_Sun_-_Cliff`)))

(event `self.ReceiveActorBeginOverlap`
  (params (OtherActor :type "Actor Object Reference"))
  (if (`self.CollectableMode`)
    (bind _asbp_top_down_player (cast `/Game/ThirdPerson/Blueprints/BP_TopDownPlayer` OtherActor))
    (`PrimitiveComponent.IgnoreActorWhenMoving` (`self.StaticMesh`) OtherActor true)
    (`PrimitiveComponent.IgnoreActorWhenMoving` (`self.Sphere`) OtherActor true)
    (`/Engine/EditorBlueprintResources/StandardMacros.DoOnce` false
      (:`Completed`
        (bind _asbp_top_downgame (cast `/Game/ThirdPerson/Blueprints/BP_TopDowngame` (`GameplayStatics.GetGameMode`)))
        (`ActorComponent.K2_DestroyComponent` (`self.Sphere`))
        (`/Game/ThirdPerson/Blueprints/BP_TopDowngame.HatCollect` _asbp_top_downgame self)
        (`self.K2_AttachToComponent` (`/Game/ThirdPerson/Blueprints/BP_TopDownPlayer.Hat` _asbp_top_down_player) "None" "SnapToTarget" "KeepRelative" "KeepRelative" false)
        (bind (_direction _newtrack_0) (`Timeline|Timeline` :!via `PlayFromStart`)
          (:`Update`
            (`AudioComponent.SetFloatParameter` (`self.001_Scene_2_-_Sun_-_Cliff`) "Fade" _newtrack_0)))))))

(event `DetachHat`
  (`SceneComponent.K2_DetachFromComponent` (`self.StaticMesh`) "KeepRelative" "KeepRelative" "KeepRelative" true))

(event `AttachToNew`
  (params (NewParam :type "Actor Object Reference"))
  (`PrimitiveComponent.IgnoreActorWhenMoving` (`self.StaticMesh`) NewParam true)
  ; Attach TO NPC
  (`self.K2_AttachToComponent` (`Actor.RootComponent` NewParam) "Hat" "SnapToTarget" "KeepRelative" "KeepRelative" false))

(fn `UserConstructionScript`)