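; LightDetector is an actor that checks line of sight to the two players and sends a die message to whatever its trace hits.
; Each Tick traces on Visibility from itself to one player character, with a FlipFlop alternating the player index.
; It prints when either player is hit, but calls DieMessage on the hit actor regardless.
; The directional light lookup never runs, and BeginPlay's enum-printing loop has no array connected.
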(event `self.ReceiveBeginPlay`
  (for _array_element _
    (`KismetSystemLibrary.PrintString` (`|GetEnumeratorNameAsString` _array_element))))

(event `self.ReceiveTick`
  (params (DeltaSeconds :type "Float (single-precision)"))
  (bind _outhit (`KismetSystemLibrary.LineTraceSingle` (`self.K2_GetActorLocation`) (`self.K2_GetActorLocation` (`GameplayStatics.GetPlayerCharacter` (`self.Player`))) "TraceTypeQuery1"))
  (if (or (== (`.HitActor` (`GameplayStatics.BreakHitResult` _outhit)) (`GameplayStatics.GetPlayerCharacter` 0)) (== (`.HitActor` (`GameplayStatics.BreakHitResult` _outhit)) (`GameplayStatics.GetPlayerCharacter` 1)))
    (`KismetSystemLibrary.PrintString` "hit player"))
  (`/Engine/EditorBlueprintResources/StandardMacros.FlipFlop`
    (:`A`
      (set `self.Player` 0))
    (:`B`
      (set `self.Player` 1)))
  (message `/Game/ThirdPerson/Blueprints/Game/BPI_Players.Die` (`.HitActor` (`GameplayStatics.BreakHitResult` _outhit)) false))

(fn `GetInteractionInstigator`
  (returns (InteractionInstigator :type "Actor Object Reference"))
  (return null))

(fn `UserConstructionScript`)