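; BP_PhysicsBlock is a block actor whose Cube can be pulled toward a supplied location through its Interact event.
; Each Interact call prints a debug message, then moves the Cube a small fixed fraction toward that location with a swept move, so repeated calls give eased, collision-aware following.
; The start location saved on BeginPlay, an axis-lock multiply, a gravity toggle and a Timeline are unused leftovers.
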(event `self.ReceiveBeginPlay`
  (set `self.Offset` (`SceneComponent.K2_GetComponentLocation` (`self.Cube`))))

(event `/Game/ThirdPerson/Blueprints/Game/BPI_Players.Interact`
  (params (Location :type "Vector Structure"))
  (`KismetSystemLibrary.PrintString` "Block is touched")
  (`SceneComponent.K2_SetWorldLocation` (`self.Cube`) (`KismetMathLibrary.VLerp` (`SceneComponent.K2_GetComponentLocation` (`self.Cube`)) Location 0.08) true false))

(fn `UserConstructionScript`)