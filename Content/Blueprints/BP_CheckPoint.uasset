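; BP_CheckPoint is a checkpoint actor for the top-down player that lights up while any player has it registered.
; On capsule overlap, each player not already in its Players array is added and told to remember this checkpoint, triggering a sound and a Timeline-driven light fade-in.
; Its RememberCheckpoint event removes a player, and once none remain the Timeline reverses to fade out and hide the light.
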(event `self.ReceiveActorBeginOverlap`
  (params (OtherActor :type "Actor Object Reference")))

(event `self.Capsule.OnComponentBeginOverlap`
  (params (OverlappedComponent :type "PrimitiveComponent Object Reference") (OtherActor :type "Actor Object Reference") (OtherComp :type "PrimitiveComponent Object Reference") (OtherBodyIndex :type Integer) (bFromSweep :type Boolean) (SweepResult :type "HitResult Structure (by ref)"))
  (bind _asbp_top_down_player (cast `/Game/ThirdPerson/Blueprints/BP_TopDownPlayer` OtherActor))
  ; Do once per player
  (if (> 0 (`KismetArrayLibrary.Array_Find` (`self.Players`) _asbp_top_down_player))
    (`KismetArrayLibrary.Array_Add` (`self.Players`) _asbp_top_down_player)
    (`/Game/ThirdPerson/Blueprints/Game/BPI_Players.RememberCheckpoint` _asbp_top_down_player self null false)
    (`SceneComponent.SetVisibility` (`self.PointLight`) true false)
    (`GameplayStatics.PlaySoundAtLocation` "/Game/Audio/SFX/UI/SawUIClose.SawUIClose" (`SceneComponent.K2_GetComponentLocation` (`self.DefaultSceneRoot`)) (struct) 1.0 1.0 0.0 null null null null)
    (bind (_direction _newtrack_0) (`Timeline|Timeline` :!label _label)
      (:`Update`
        (`LightComponent.SetIntensity` (`self.PointLight`) (* _newtrack_0 5000.0)))
      (:`Finished`
        (switch `ETimelineDirection` _direction
          (:`Backward`
            (`SceneComponent.SetVisibility` (`self.PointLight`) false false)))))))

(event `/Game/ThirdPerson/Blueprints/Game/BPI_Players.RememberCheckpoint`
  (params (Checkpoint :type "/Game/Blueprints/BP_CheckPoint Object Reference") (Player :type "/Game/ThirdPerson/Blueprints/BP_TopDownPlayer Object Reference") (Manual :type Boolean))
  ; Player is Cheating on me
  (`KismetArrayLibrary.Array_RemoveItem` (`self.Players`) Player)
  ; Does no one love me
  (if (not (> (`KismetArrayLibrary.Array_Length` (`self.Players`)) 0))
    (goto _label :!via `ReverseFromEnd`)))

(fn `UserConstructionScript`
  (bind _pointlight (`self.PointLight`))
  (`LightComponent.SetIntensity` _pointlight 0.0)
  (`SceneComponent.SetVisibility` _pointlight false false))