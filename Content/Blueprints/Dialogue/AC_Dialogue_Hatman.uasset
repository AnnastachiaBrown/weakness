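; Dialogue component for the Hatman character, overriding Dialogue to define a short branching conversation about question marks.
; A switch on the dialogue tree index selects the tree, with nested AddDialogue nodes branching on the chosen option.
; Endings close the conversation and either advance to the second tree, partially roll back progress or clear it.
; The second tree shows one of two random lines, then clears progress on leaving.
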(fn `Dialogue`
  (`parent.Dialogue`)
  (switch `int` (`self.DialogueTreeIndex`)
    (:`0`
      (bind (_state _optionindex) (`self.AddDialogue` "Hatman" "Hi, this is a question." (`|MakeArray` "Yes" "No" :!type "Text")))
      (switch `/Game/Blueprints/Dialogue/E_DialogueState` _state
        (:`NewEnumerator0`
          (switch `int` _optionindex
            (:`0`
              (bind (_state_2 _optionindex_2) (`self.AddDialogue` "Hatman" "Glad you agree, but there wasn't a question mark. This one does though?" (`|MakeArray` "Yeah but you aren't asking me anything." "Confusing stuff..." :!type "Text")))
              (switch `/Game/Blueprints/Dialogue/E_DialogueState` _state_2
                (:`NewEnumerator0`
                  (switch `int` _optionindex_2
                    (:`0`
                      (bind _state_3 (`self.AddDialogue` "Hatman" "You make a good point." (`|MakeArray` "Leave" :!type "Text")))
                      (switch `/Game/Blueprints/Dialogue/E_DialogueState` _state_3
                        (:`NewEnumerator0`
                          (`self.SetDialogueTreeIndex` 1)
                          (`self.CloseConversation`))))
                    (:`1`
                      (bind _state_4 (`self.AddDialogue` "Hatman" "Right?" (`|MakeArray` "Leave" :!type "Text")))
                      (switch `/Game/Blueprints/Dialogue/E_DialogueState` _state_4
                        (:`NewEnumerator0`
                          (`self.RemoveDialogueProgress` 2)
                          (`self.CloseConversation`))))))))
            (:`1`
              (bind _state_5 (`self.AddDialogue` "Hatman" "Right, forgot the question mark." (`|MakeArray` "Leave" :!type "Text")))
              (switch `/Game/Blueprints/Dialogue/E_DialogueState` _state_5
                (:`NewEnumerator0`
                  (`self.ClearDialogueProgress`)
                  (`self.CloseConversation`))))))))
    (:`1`
      (bind _state_6 (`self.AddDialogue` "Hatman" (select `int` (`KismetMathLibrary.RandomIntegerInRange` 0 1) :`0` "Oh, you're still here?" :`1` "..." :!type "Text") (`|MakeArray` "Leave" :!type "Text")))
      (switch `/Game/Blueprints/Dialogue/E_DialogueState` _state_6
        (:`NewEnumerator0`
          (`self.ClearDialogueProgress`)
          (`self.CloseConversation`))))))