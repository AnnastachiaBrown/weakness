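; Dialogue component holding the story conversations between Iru and Vekka, from the game's opening through finding each of four hats.
; RunDialogue opens the conversation and switches the player to UI-only input with a visible cursor.
; An overridden Dialogue function switches on the active branch, chains single-option lines, then advances to the next hat's branch and closes.
; The opening branch also notifies the top-down player on close, while the last clears dialogue progress.
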(event `self.ReceiveBeginPlay`
  (bind _asbp_top_down_player (cast `/Game/ThirdPerson/Blueprints/BP_TopDownPlayer` (`GameplayStatics.GetPlayerCharacter` 0)))
  (set `self.BP_TopDownPlayer Ref` _asbp_top_down_player))

(event `RunDialogue`
  (`self.OpenConversation`)
  (`WidgetBlueprintLibrary.SetInputMode_UIOnlyEx` (`GameplayStatics.GetPlayerController` 0) null)
  (set `PlayerController.bShowMouseCursor` true (`GameplayStatics.GetPlayerController` 0)))

(fn `Dialogue`
  ;[0.15 0.05536 0.05038 0.5] Switch on branch
  (`parent.Dialogue`)
  (switch `name` (`self.ActiveDialogueBranch`)
    (:`Beginning`
      ; Beginning of the game
      (bind _state (`self.AddDialogue` "Iru" "We better hurry! The sun is coming out!" (`|MakeArray` ">" :!type "Text")))
      (switch `/Game/Blueprints/Dialogue/E_DialogueState` _state
        (:`NewEnumerator0`
          (bind _state_2 (`self.AddDialogue` "Vekka" "Right behind you!" (`|MakeArray` ">" :!type "Text")))
          (switch `/Game/Blueprints/Dialogue/E_DialogueState` _state_2
            (:`NewEnumerator0`
              (`self.SetDialogueBranch` "FirstHat")
              (`self.CloseConversation`)
              (`/Game/ThirdPerson/Blueprints/BP_TopDownPlayer.ConversationClosed` (`self.BP_TopDownPlayer Ref`)))))))
    (:`FirstHat`
      ; Found the first hat
      (bind _state_3 (`self.AddDialogue` "Iru" "Here's the first hat. We'd better get back and give it to the crazy nuthead." (`|MakeArray` ">" :!type "Text")))
      (switch `/Game/Blueprints/Dialogue/E_DialogueState` _state_3
        (:`NewEnumerator0`
          (bind _state_4 (`self.AddDialogue` "Vekka" "Let's hurry, I can't wait for my bed." (`|MakeArray` ">" :!type "Text")))
          (switch `/Game/Blueprints/Dialogue/E_DialogueState` _state_4
            (:`NewEnumerator0`
              (`self.SetDialogueBranch` "SecondHat")
              (`self.CloseConversation`))))))
    (:`SecondHat`
      ; Found the second hat
      (bind _state_5 (`self.AddDialogue` "Vekka" "Here's the second hat! I'm so tired, I just want to go back already." (`|MakeArray` ">" :!type "Text")))
      (switch `/Game/Blueprints/Dialogue/E_DialogueState` _state_5
        (:`NewEnumerator0`
          (bind _state_6 (`self.AddDialogue` "Iru" "Finally, we only have two left." (`|MakeArray` ">" :!type "Text")))
          (switch `/Game/Blueprints/Dialogue/E_DialogueState` _state_6
            (:`NewEnumerator0`
              (`self.SetDialogueBranch` "ThirdHat")
              (`self.CloseConversation`))))))
    (:`ThirdHat`
      ; Found the third hat
      (bind _state_7 (`self.AddDialogue` "Iru" "The third hat... here we go again with his jokes." (`|MakeArray` ">" :!type "Text")))
      (switch `/Game/Blueprints/Dialogue/E_DialogueState` _state_7
        (:`NewEnumerator0`
          (bind _state_8 (`self.AddDialogue` "Vekka" "I don't think I can listen to another one of his jokes." (`|MakeArray` ">" :!type "Text")))
          (switch `/Game/Blueprints/Dialogue/E_DialogueState` _state_8
            (:`NewEnumerator0`
              (`self.SetDialogueBranch` "FourthHat")
              (`self.CloseConversation`))))))
    (:`FourthHat`
      ; Found the fourth hat
      (bind _state_9 (`self.AddDialogue` "Iru" "How strange... well, this is the last hat." (`|MakeArray` ">" :!type "Text")))
      (switch `/Game/Blueprints/Dialogue/E_DialogueState` _state_9
        (:`NewEnumerator0`
          (bind _state_10 (`self.AddDialogue` "Vekka" "What do you mean strange?" (`|MakeArray` ">" :!type "Text")))
          (switch `/Game/Blueprints/Dialogue/E_DialogueState` _state_10
            (:`NewEnumerator0`
              (bind _state_11 (`self.AddDialogue` "Iru" "I can't explain it but it feels different." (`|MakeArray` ">" :!type "Text")))
              (switch `/Game/Blueprints/Dialogue/E_DialogueState` _state_11
                (:`NewEnumerator0`
                  (`self.ClearDialogueProgress`)
                  (`self.CloseConversation`))))))))))

(fn `GetInteractionInstigator`
  (returns (InteractionInstigator :type "Actor Object Reference"))
  (return null))

(fn `OpenConversation`
  ; Branch Check
  (switch `name` (`self.ActiveDialogueBranch`)
    (:`Beginning`
      (`self.SetDialogueBranch` "Beginning")
      (`KismetSystemLibrary.PrintString` "Reached branch: Beginning" true true (struct :`R` 0.904661 :`B` 1.0 :`A` 1.0)))
    (:`FirstHat`
      (`self.SetDialogueBranch` "FirstHat")
      (`KismetSystemLibrary.PrintString` "Reached branch: FirstHat" true true (struct :`R` 0.904661 :`B` 1.0 :`A` 1.0)))
    (:`SecondHat`
      (`self.SetDialogueBranch` "SecondHat")
      (`KismetSystemLibrary.PrintString` "Reached branch: SecondHat" true true (struct :`R` 0.904661 :`B` 1.0 :`A` 1.0)))
    (:`ThirdHat`
      (`self.SetDialogueBranch` "ThirdHat")
      (`KismetSystemLibrary.PrintString` "Reached branch: ThirdHat" true true (struct :`R` 0.904661 :`B` 1.0 :`A` 1.0)))
    (:`FourthHat`
      (`self.SetDialogueBranch` "FourthHat")
      (`KismetSystemLibrary.PrintString` "Reached branch: FourthHat" true true (struct :`R` 0.904661 :`B` 1.0 :`A` 1.0))))
  (`parent.OpenConversation`))