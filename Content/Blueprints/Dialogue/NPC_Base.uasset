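; NPC_Base is a base Blueprint for dialogue NPCs that shows a character name label and reports when a conversation ends.
; The construction script fills the TxtCharacterName component from the CharacterName variable.
; SetInteractableState toggles that label's visibility based on whether interaction can be shown.
; ConversationClosed forwards a ConversationClosedMessage to the stored InteractInstigator.
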(event `/Game/ThirdPerson/Blueprints/Game/BPI_Players.SetInteractableState`
  (params (`CanShowInteract?` :type Boolean))
  (if `CanShowInteract?`
    (`SceneComponent.SetVisibility` (`self.Txt_CharacterName`) true false)
    (else
      (`SceneComponent.SetVisibility` (`self.Txt_CharacterName`) false false))))

(event `/Game/ThirdPerson/Blueprints/Game/BPI_Players.ConversationClosed`
  (message `/Game/ThirdPerson/Blueprints/Game/BPI_Players.ConversationClosed` (`self.InteractInstigator`)))

(fn `UserConstructionScript`
  (`TextRenderComponent.K2_SetText` (`self.Txt_CharacterName`) (`self.CharacterName`)))