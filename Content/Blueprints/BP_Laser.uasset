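; BP_Laser is a laser beam actor that traces forward every tick, stretching its colored mesh to the blocking hit.
; Hit actors' AC_Handler components receive start and stop messages by diffing hit sets between frames, but only when the trace reports a blocking hit.
; LaserStopHitting notifies previous handlers and destroys the beam.
; IsNotOnPath should filter upstream handlers, but its disconnected comparison rejects every handler whenever previous lasers exist.
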(event `self.ReceiveBeginPlay`
  (bind _returnvalue (`KismetMaterialLibrary.CreateDynamicMaterialInstance` "/Game/Materials/MI_laser.MI_laser"))
  (set `self.MaterialInstance` _returnvalue)
  (`PrimitiveComponent.SetMaterial` (`self.StaticMesh`) 0 (`self.MaterialInstance`))
  (`self.ChangeLaserColor` (`self.ColorOverride`)))

(event `self.ReceiveTick`
  (params (DeltaSeconds :type "Float (single-precision)"))
  (bind _returnvalue (`self.K2_GetActorLocation`))
  (bind (_outhits _returnvalue_2) (`KismetSystemLibrary.LineTraceMulti` _returnvalue (+ _returnvalue (* (`self.GetActorForwardVector`) (`self.Range`))) "TraceTypeQuery1" false (`self.Actors to Ingore`) "ForOneFrame"))
  (if _returnvalue_2
    (for _array_element _outhits
      (`|ExecutionSequence`
        (:`then_0`
          (bind (_bblockinghit _binitialoverlap _time _distance) (`GameplayStatics.BreakHitResult` _array_element))
          (if _bblockinghit
            (`self.UpdateLength` _distance)))
        (:`then_1`
          (`self.HandleHitActor` _array_element))))
    (bind _result (`BlueprintSetLibrary.Set_Difference` (`self.PreviouslyHitHandles`) (`self.CurrentHitHandlers`)))
    (bind _result_2 (`BlueprintSetLibrary.Set_ToArray` _result))
    (for _array_element_2 _result_2
      (message `/Game/Blueprints/BPI_Lasers.LaserStopHitting` _array_element_2 self)
      (`BlueprintMapLibrary.Map_Remove` (`self.HittingHandlers`) _array_element_2))
    (set `self.PreviouslyHitHandles` (`self.CurrentHitHandlers`))
    (`BlueprintSetLibrary.Set_Clear` (`self.CurrentHitHandlers`))
    (else
      (`self.UpdateLength` (`self.Range`)))))

(event `/Game/Blueprints/BPI_Lasers.LaserStopHitting`
  (params (Input :type "/Game/Blueprints/BP_Laser Object Reference"))
  (`|ExecutionSequence`
    (:`then_0`
      (bind _result (`BlueprintSetLibrary.Set_ToArray` (`self.PreviouslyHitHandles`)))
      (for _array_element _result
        (message `/Game/Blueprints/BPI_Lasers.LaserStopHitting` _array_element self)))
    (:`then_1`
      (`self.K2_DestroyActor`))))

(fn `ChangeLaserColor`
  (params (Value :type "LinearColor Structure"))
  (`MaterialInstanceDynamic.SetVectorParameterValue` (`self.MaterialInstance`) "Color" Value))

(fn `HandleHitActor`
  (params (InputPin :type "HitResult Structure"))
  (bind _returnvalue (`self.GetComponentByClass` (`.HitActor` (`GameplayStatics.BreakHitResult` InputPin)) "/Game/Blueprints/AC_Handler.AC_Handler_C"))
  (`/Engine/EditorBlueprintResources/StandardMacros.IsValid` _returnvalue
    (:`Is Valid`
      (set `self.L-Handler` _returnvalue)
      (if (`self.IsNotOnPath` (`self.L-Handler`))
        (`BlueprintMapLibrary.Map_Add` (`self.HittingHandlers`) (`self.L-Handler`) (`local.InputPin`))
        (if (not (`BlueprintSetLibrary.Set_Contains` (`self.PreviouslyHitHandles`) (`self.L-Handler`)))
          (message `/Game/Blueprints/BPI_Lasers.LaserStartHitting` (`self.L-Handler`) self (`local.InputPin`)))
        (`BlueprintSetLibrary.Set_Add` (`self.CurrentHitHandlers`) (`self.L-Handler`))))))

(fn `IsNotOnPath`
  (params (InputHandler :type "/Game/Blueprints/AC_Handler Object Reference"))
  (returns (OutputPin :type Boolean))
  (if (`KismetArrayLibrary.Array_IsNotEmpty` (`self.PrevoiusLasers`))
    (for _array_element (`self.PrevoiusLasers`)
      (bind _output_get (set `self.L-Current Laser` _array_element))
      (if true
        (return false)
        (elif (not (`self.IsNotOnPath` (`self.L-Current Laser`) (`local.InputHandler`)))
          (return false))))
    (return true)
    (else
      (return true))))

(fn `UpdateLength`
  (params (InputPin :type "Float (single-precision)"))
  (if (not (`KismetMathLibrary.NearlyEqual_FloatFloat` InputPin (`self.PreviousLength`) 2.0))
    (bind _output_get (set `self.PreviousLength` (`local.InputPin`)))
    (`SceneComponent.SetWorldScale3D` (`self.StaticMesh`) (`KismetMathLibrary.MakeVector` 0.1 0.1 (/ _output_get 100.0)))))

(fn `UserConstructionScript`)