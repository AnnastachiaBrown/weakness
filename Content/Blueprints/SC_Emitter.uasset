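; SC_Emitter is a scene component that emits a laser beam in response to laser hit start and stop events.
; It caches the owner's AC_Handler, then spawns BP_Laser at its transform with color, range, previous lasers and handler, attaching it to itself.
; Deactivation forwards LaserStopHitting to that laser.
; An inversion check swaps activate and deactivate, though ISSystemInverted and GetFilteredLasers show only unused handler reads.
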(event `self.ReceiveBeginPlay`
  (bind _returnvalue (`Actor.GetComponentByClass` (`self.GetOwner`) "/Game/Blueprints/AC_Handler.AC_Handler_C"))
  (`/Engine/EditorBlueprintResources/StandardMacros.IsValid` _returnvalue
    (:`Is Valid`
      (set `self.OwningHandler` _returnvalue))))

(event `/Game/Blueprints/BPI_Lasers.LaserStartHitting`
  (params (Input :type "/Game/Blueprints/BP_Laser Object Reference") (HitInput :type "HitResult Structure"))
  (if (`self.ISSystemInverted`)
    (`self.Deactivate Laser`)
    (else
      (`self.ActivateLaser`))))

(event `/Game/Blueprints/BPI_Lasers.LaserStopHitting`
  (params (Input :type "/Game/Blueprints/BP_Laser Object Reference"))
  (if (`self.ISSystemInverted`)
    (`self.ActivateLaser`)
    (else
      (`self.Deactivate Laser`))))

(fn `ActivateLaser`
  (bind _returnvalue (`|SpawnActorFromClass` "/Game/Blueprints/BP_Laser.BP_Laser_C" (`self.K2_GetComponentToWorld`) "Undefined" "MultiplyWithRoot" null (`self.CurrentColor`) (`self.Max Range`) (`self.GetFilteredLasers`) (`self.OwningHandler`) (`|MakeArray` (`self.GetOwner`)) null))
  (bind _output_get (set `self.Attached Laser` _returnvalue))
  (`Actor.K2_AttachToComponent` _output_get self "None" "KeepWorld" "KeepWorld" "KeepWorld" false))

(fn `Deactivate Laser`
  (bind _attached_laser (`self.Attached Laser`)
    (:`then`
      (`/Game/Blueprints/BP_Laser.LaserStopHitting` _attached_laser null))
    (:`else`)))