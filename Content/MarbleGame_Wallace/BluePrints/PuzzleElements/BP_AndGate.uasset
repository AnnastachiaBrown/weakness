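; BP_AndGate is a puzzle element that acts as a logical AND gate, firing its targets once enough inputs are active.
; Activate increments a counter and Reset decrements it; reaching the NumperOfInputs threshold calls Activate on every actor in the Target array.
; A DoOnce that is never reset limits this to a single firing, even if the count drops afterwards.
; Its Cube is hidden on BeginPlay and has no collision.
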(event `self.ReceiveBeginPlay`
  (set `self.I` 0)
  (`SceneComponent.SetVisibility` (`self.Cube`) false false))

(event `self.Activate`
  (`/Engine/EditorBlueprintResources/StandardMacros.IncrementInt` (`self.I`)
    (:`  `
      (if (>= (`self.I`) (`self.NumperOfInputs`))
        (`/Engine/EditorBlueprintResources/StandardMacros.DoOnce` false
          (:`Completed`
            (for _array_element (`self.Target`)
              (`self.Activate` _array_element))))))))

(event `self.Reset`
  (`/Engine/EditorBlueprintResources/StandardMacros.DecrementInt` (`self.I`)))

(fn `UserConstructionScript`
  (`PrimitiveComponent.SetCollisionEnabled` (`self.Cube`) "NoCollision"))