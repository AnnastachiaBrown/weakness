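; BP_PB_LazerEnd2 is a laser receiver puzzle element that activates its TargetElement while a laser hits it and resets it when the laser leaves.
; Each Tick it checks whether any BP_Laser actor overlaps its Box.
; Two DoOnce nodes re-arm each other, so Activate and Reset each fire only once per change of state.
; The construction script destroys the inherited Button component.
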(event `self.Box.OnComponentBeginOverlap`
  (params (OverlappedComponent :type "PrimitiveComponent Object Reference") (OtherActor :type "Actor Object Reference") (OtherComp :type "PrimitiveComponent Object Reference") (OtherBodyIndex :type Integer) (bFromSweep :type Boolean) (SweepResult :type "HitResult Structure (by ref)")))

(event `self.ReceiveTick`
  (params (DeltaSeconds :type "Float (single-precision)"))
  (if (> (`KismetArrayLibrary.Array_Length` (`PrimitiveComponent.GetOverlappingActors` (`self.Box`) "/Game/Blueprints/BP_Laser.BP_Laser_C")) 0)
    (`|ExecutionSequence`
      (:`then_0`
        (`/Engine/EditorBlueprintResources/StandardMacros.DoOnce` false :!label _label
          (:`Completed`
            (`/Game/MarbleGame_Wallace/BluePrints/PuzzleElements/BP_Element.Activate` (`self.TargetElement`)))))
      (:`then_1`
        (goto _label_2 :!via `Reset`)))
    (else
      (`|ExecutionSequence`
        (:`then_0`
          (`/Engine/EditorBlueprintResources/StandardMacros.DoOnce` false :!label _label_2
            (:`Completed`
              (`/Game/MarbleGame_Wallace/BluePrints/PuzzleElements/BP_Element.Reset` (`self.TargetElement`)))))
        (:`then_1`
          (goto _label :!via `Reset`))))))

(fn `UserConstructionScript`
  (`parent.UserConstructionScript`)
  (`ActorComponent.K2_DestroyComponent` (`self.Button`)))