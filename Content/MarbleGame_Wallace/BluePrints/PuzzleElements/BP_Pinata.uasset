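; BP_Pinata is a puzzle-element actor that bursts into physics coins as soon as it begins play, then destroys itself.
; BeginPlay plays a sound, then a delay-driven loop spawns BP_Coin_Phys actors one at a time up to the configured count.
; Each coin gets a random material and upward launch velocity with sideways scatter, then receives its index through OnSpawn.
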(event `self.ReceiveBeginPlay`
  (bind _num (`self.Num`))
  (`/Engine/EditorBlueprintResources/StandardMacros.DoOnce` false
    (:`Completed`
      (`GameplayStatics.PlaySoundAtLocation` null (0.0 0.0 0.0) (struct) 0.3 0.5 0.0 null null null null)
      (set `self.Num` 0)
      (if (< (`self.Num`) (`self.NumperOfCoins`)) :!label _label
        (`/Engine/EditorBlueprintResources/StandardMacros.IncrementInt` (`self.Num`)
          (:`  `
            (bind _returnvalue (`|SpawnActorFromClass` "/Game/MarbleGame_Wallace/BluePrints/PuzzleElements/BP_Coin_Phys.BP_Coin_Phys_C" (`SceneComponent.GetRelativeTransform` (`self.DefaultSceneRoot`)) "AlwaysSpawn" "MultiplyWithRoot" null null))
            (bind _coin (`/Game/MarbleGame_Wallace/BluePrints/PuzzleElements/BP_Coin_Phys.Coin` _returnvalue))
            (`PrimitiveComponent.SetMaterial` _coin 0 (`KismetArrayLibrary.Array_Random` (`self.Materials`)))
            (`PrimitiveComponent.SetPhysicsLinearVelocity` _coin (`KismetMathLibrary.MakeVector` (`KismetMathLibrary.RandomFloatInRange` -60.0 60.0) (`KismetMathLibrary.RandomFloatInRange` -60.0 60.0) (`KismetMathLibrary.RandomFloatInRange` 600.0 800.0)) false "None")
            (`/Game/MarbleGame_Wallace/BluePrints/PuzzleElements/BP_Coin_Phys.On Spawn` _returnvalue (`KismetMathLibrary.Conv_IntToDouble` _num))
            (`KismetSystemLibrary.PrintString` (`KismetStringLibrary.Conv_IntToString` _num))
            (`KismetSystemLibrary.Delay` (`self.Wait time`))
            (goto _label)))
        (else
          (`self.K2_DestroyActor`))))))

(fn `UserConstructionScript`)