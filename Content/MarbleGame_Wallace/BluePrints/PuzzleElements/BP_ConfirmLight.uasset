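; BP_ConfirmLight is a puzzle element actor in the marble game that serves as an indicator light.
; Its PointLight starts hidden, set both in the construction script and on BeginPlay.
; The Activate event shows the light and the Reset event hides it again; nothing in this Blueprint calls either event.
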(event `self.ReceiveBeginPlay`
  (`SceneComponent.SetVisibility` (`self.PointLight`) false false))

(event `self.ReceiveActorBeginOverlap`
  (params (OtherActor :type "Actor Object Reference")))

(event `self.ReceiveTick`
  (params (DeltaSeconds :type "Float (single-precision)")))

(event `self.Activate`
  (`SceneComponent.SetVisibility` (`self.PointLight`) true false))

(event `self.Reset`
  (`SceneComponent.SetVisibility` (`self.PointLight`) false false))

(fn `UserConstructionScript`
  (`SceneComponent.SetVisibility` (`self.PointLight`) false false))