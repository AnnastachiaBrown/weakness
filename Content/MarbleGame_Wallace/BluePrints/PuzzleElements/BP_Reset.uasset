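; BP_Reset is a puzzle element that resets a linked target element when a qualifying actor overlaps it.
; The LookForBall flag selects whether it responds to a toy ball or physics block, or instead to the top-down player.
; On a matching overlap it calls Activate, then calls Reset on TargetElement.
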(event `self.ReceiveActorBeginOverlap`
  (params (OtherActor :type "Actor Object Reference"))
  (if (`self.LookForBall`)
    (cast `/Game/MarbleGame_Wallace/BluePrints/PuzzleElements/BP_ToyBall` OtherActor
      (:`then`
        _)
      (:`CastFailed`
        (cast `/Game/Blueprints/BP_PhysicsBlock` OtherActor)))
    (else
      (cast `/Game/ThirdPerson/Blueprints/BP_TopDownPlayer` OtherActor)))
  (`self.Activate`)
  (`/Game/MarbleGame_Wallace/BluePrints/PuzzleElements/BP_Element.Reset` (`self.TargetElement`)))

(fn `UserConstructionScript`
  (`parent.UserConstructionScript`))