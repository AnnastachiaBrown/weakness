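; BP_PushVolume is a puzzle element that pushes toy balls (BP_ToyBall) inside its volume along an arrow's direction.
; A ball entering the volume sets a Listening flag, so Tick only does work while balls are present.
; Each tick it applies a velocity-change impulse of PushForce along the Arrow's forward vector to every overlapping ball, not scaled by delta time, and clears the flag once none remain.
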(event `self.ReceiveActorBeginOverlap`
  (params (OtherActor :type "Actor Object Reference"))
  (cast `/Game/MarbleGame_Wallace/BluePrints/PuzzleElements/BP_ToyBall` OtherActor)
  (set `self.Listening` true))

(event `self.ReceiveTick`
  (params (DeltaSeconds :type "Float (single-precision)"))
  (bind _overlappingactors (`self.GetOverlappingActors` "/Game/MarbleGame_Wallace/BluePrints/PuzzleElements/BP_ToyBall.BP_ToyBall_C"))
  ; is there two players
  (if (`self.Listening`)
    (if (> (`KismetArrayLibrary.Array_Length` _overlappingactors) 0)
      (for _array_element _overlappingactors
        (`PrimitiveComponent.AddImpulse` (`/Game/MarbleGame_Wallace/BluePrints/PuzzleElements/BP_ToyBall.Collision` _array_element) (* (`SceneComponent.GetForwardVector` (`self.Arrow`)) (`self.PushForce`)) "None" true))
      (else
        (set `self.Listening` false)))))

(fn `UserConstructionScript`)