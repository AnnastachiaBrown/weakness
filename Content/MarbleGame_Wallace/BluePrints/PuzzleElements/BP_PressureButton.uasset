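; Pressure button puzzle element that activates its linked TargetElement when something overlaps its trigger box.
; LookForBall selects what can trigger it: either a toy ball or physics block, or the top-down player.
; Activation plays a sound and, with DoColorToggle on, swaps the button material for a second before restoring it.
; The construction script applies the Visible setting and the default button material.
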(event `self.Box.OnComponentBeginOverlap`
  (params (OverlappedComponent :type "PrimitiveComponent Object Reference") (OtherActor :type "Actor Object Reference") (OtherComp :type "PrimitiveComponent Object Reference") (OtherBodyIndex :type Integer) (bFromSweep :type Boolean) (SweepResult :type "HitResult Structure (by ref)"))
  (if (`self.LookForBall`)
    (cast `/Game/MarbleGame_Wallace/BluePrints/PuzzleElements/BP_ToyBall` OtherActor
      (:`then`
        _)
      (:`CastFailed`
        (cast `/Game/Blueprints/BP_PhysicsBlock` OtherActor)))
    (else
      (cast `/Game/ThirdPerson/Blueprints/BP_TopDownPlayer` OtherActor)))
  (`self.Activate`)
  (`/Game/MarbleGame_Wallace/BluePrints/PuzzleElements/BP_Element.Activate` (`self.TargetElement`)))

(event `Activate`
  (bind _button (`self.Button`))
  (`GameplayStatics.PlaySoundAtLocation` "/Game/Audio/SFX/ToyBarrelLoad.ToyBarrelLoad" (`SceneComponent.K2_GetComponentLocation` (`self.DefaultSceneRoot`)) (struct) 1.0 1.0 0.0 null null null null)
  (if (`self.DoColorToggle`)
    (`PrimitiveComponent.SetMaterial` _button 0 null) ; Change the color of the platform to "Activated"
    (`KismetSystemLibrary.Delay` 1.0)
    (`PrimitiveComponent.SetMaterial` _button 0 (`self.Material`)) ; Change the color of the platform to "Activated"
  ))

(fn `UserConstructionScript`
  (`SceneComponent.SetVisibility` (`self.Button`) (`self.Visible`) false)
  (set `self.Material` "/Game/Materials/Parent/MI_Button.MI_Button")
  (`PrimitiveComponent.SetMaterial` (`self.Button`) 0 (`self.Material`)))