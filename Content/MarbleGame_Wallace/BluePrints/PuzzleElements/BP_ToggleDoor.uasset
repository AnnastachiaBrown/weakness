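; BP_ToggleDoor is a puzzle-element door for the marble game that swings open and closed by yawing its Cube mesh.
; BeginPlay caches the Cube's relative transform as the closed pose.
; Activate plays a timeline that adds up to 90 degrees of yaw to that cached rotation, and Reset reverses it.
; Older DoOnce-based toggle logic remains in the graph but is disconnected and never runs.
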(event `self.ReceiveBeginPlay`
  (`parent.ReceiveBeginPlay`)
  (set `self.OriginalTransform` (`SceneComponent.GetRelativeTransform` (`self.Cube`))))

(event `self.ReceiveActorBeginOverlap`
  (params (OtherActor :type "Actor Object Reference")))

(event `self.Activate`
  (bind (_originaltransform_location _originaltransform_rotation) (`KismetMathLibrary.BreakTransform` (`self.OriginalTransform`)))
  (bind (_direction _newtrack_1) (`Timeline|Timeline` :!label _label)
    (:`Update`
      (`SceneComponent.K2_SetRelativeRotation` (`self.Cube`) (`KismetMathLibrary.ComposeRotators` _originaltransform_rotation (`KismetMathLibrary.MakeRotator` 0.0 0.0 (* _newtrack_1 90.0))) false false))))

(event `self.Reset`
  (goto _label :!via `Reverse`))

(fn `UserConstructionScript`
  (`parent.UserConstructionScript`))