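; BP_Coin_Phys is a coin puzzle element that flies into the player and vanishes as soon as play begins.
; BeginPlay disables physics and collision, plays a coin sound, then runs a timeline that pulls the coin toward the pawn while shrinking it from its construction-time scale, destroying it afterward.
; OnSpawn plays a pitch-offset ping and calls Collect after a delay, but Collect is empty and the AutoCollect branch is unconnected.
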(event `Collect`)

(event `self.ReceiveBeginPlay`
  (bind _coin (`self.Coin`))
  (bind _returnvalue (`self.K2_GetActorLocation` (`GameplayStatics.GetPlayerPawn` 0)))
  (`PrimitiveComponent.SetSimulatePhysics` (`self.Coin`) false)
  (`PrimitiveComponent.SetCollisionEnabled` (`self.Capsule`) "NoCollision")
  (`PrimitiveComponent.SetCollisionEnabled` (`self.Coin`) "NoCollision")
  (`GameplayStatics.PlaySoundAtLocation` "/Game/Audio/SFX/Coin.Coin" _returnvalue (struct) 0.1 1.0 0.0 null null null null)
  (bind (_direction _newtrack_1) (`Timeline|Timeline_0` :!via `PlayFromStart`)
    (:`Update`
      (`SceneComponent.K2_SetWorldLocation` _coin (`KismetMathLibrary.VLerp` (`SceneComponent.K2_GetComponentLocation` (`self.Coin`)) _returnvalue _newtrack_1) false false)
      (`SceneComponent.SetRelativeScale3D` _coin (* (`KismetMathLibrary.Conv_DoubleToVector` (- 1.0 _newtrack_1)) (`self.Relative Scale 3D`))))
    (:`Finished`
      (`self.K2_DestroyActor`))))

(event `On Spawn`
  (params (PitchOffset :type "Float (double-precision)"))
  (`GameplayStatics.PlaySoundAtLocation` "/Engine/EngineSounds/1kSineTonePing.1kSineTonePing" (0.0 0.0 0.0) (struct) 0.2 (+ (* PitchOffset 2.0) 2.0) 0.0 null null null null)
  (`KismetSystemLibrary.Delay` 1.0)
  (`self.Collect`))

(fn `UserConstructionScript`
  (set `self.Relative Scale 3D` (`SceneComponent.RelativeScale3D` (`self.Coin`))))