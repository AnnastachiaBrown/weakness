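; Puzzle trigger in the marble game that activates a target element while occupied and resets it when vacated.
; Tick, throttled by a short Delay, polls the Box for overlapping top-down players or physics blocks.
; Two cross-resetting DoOnce gates turn the polled state into single Activate and Reset calls on TargetElement.
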(event `self.ReceiveTick`
  (params (DeltaSeconds :type "Float (single-precision)"))
  (bind _box (`self.Box`))
  (`parent.ReceiveTick` DeltaSeconds)
  (`KismetSystemLibrary.Delay` 0.2)
  (if (or (> (`KismetArrayLibrary.Array_Length` (`PrimitiveComponent.GetOverlappingActors` _box "/Game/ThirdPerson/Blueprints/BP_TopDownPlayer.BP_TopDownPlayer_C")) 0) (> (`KismetArrayLibrary.Array_Length` (`PrimitiveComponent.GetOverlappingActors` _box "/Game/Blueprints/BP_PhysicsBlock.BP_PhysicsBlock_C")) 0))
    (`|ExecutionSequence`
      (:`then_0`
        (`/Engine/EditorBlueprintResources/StandardMacros.DoOnce` false :!label _label
          (:`Completed`
            (`/Game/MarbleGame_Wallace/BluePrints/PuzzleElements/BP_Element.Activate` (`self.TargetElement`)))))
      (:`then_1`
        (goto _label_2 :!via `Reset`)))
    (else
      (`|ExecutionSequence`
        (:`then_0`
          (`/Engine/EditorBlueprintResources/StandardMacros.DoOnce` false :!label _label_2
            (:`Completed`
              (`/Game/MarbleGame_Wallace/BluePrints/PuzzleElements/BP_Element.Reset` (`self.TargetElement`)))))
        (:`then_1`
          (goto _label :!via `Reset`))))))

(fn `UserConstructionScript`
  (`parent.UserConstructionScript`))